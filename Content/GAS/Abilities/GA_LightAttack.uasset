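; GA_LightAttack is a Gameplay Ability for a light melee attack with a forward lunge.
; On activation it asks the AnimInstance to play a combo montage and overrides horizontal velocity along the owner's forward vector, keeping vertical velocity.
; It waits for two gameplay events: Weapon.Hit applies GE_Damage to the payload's target and ends the ability, while Weapon.Swinged just ends it.
; OnEndAbility ends both wait tasks when both are valid.
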(event Ability|EventActivateAbility
  (bind _returnvalue (Ability|GetActorInfo))
  (bind _attack_laung_speed (Variables|Default|GetAttack_laung_Speed))
  (bind _returnvalue_2 (Transformation|GetActorForwardVector (.owneractor _returnvalue)))
  (bind _returnvalue_3 (* _returnvalue_2 _attack_laung_speed))
  (Class|BPIPlayMontage|PlayComboMontage(Message) (Components|SkeletalMesh|GetAnimInstance (.skeletalmeshcomponent _returnvalue)) "NewEnumerator0")
  (bind _output_get (Variables|Default|SetPlayer%20Movement%20Component (.movementcomponent _returnvalue)))
  (Variables|/Script/Engine.MovementComponent|SetVelocity _output_get (Math|Vector|MakeVector (.x _returnvalue_3) (.y _returnvalue_3) (.z (Variables|/Script/Engine.MovementComponent|GetVelocity _output_get))))
  (bind (_asynctaskproxy _payload) (Ability|Tasks|WaitGameplayEvent "(TagName=\"Weapon.Hit\")" 0 true)
    (:then
      (Variables|Default|SetHitAsync%20Task _asynctaskproxy)
      (bind _asynctaskproxy_2 (Ability|Tasks|WaitGameplayEvent "(TagName=\"Weapon.Swinged\")" 0 true)
        (:then
          (Variables|Default|SetSwingAsync%20Task _asynctaskproxy_2))
        (:EventReceived
          (Ability|EndAbility))))
    (:EventReceived
      (GameplayEffects|ApplyGameplayEffectToTarget (.TargetData (Utilities|Struct|BreakGameplayEventData _payload)) "/Game/GAS/Effects/GE_Damage.GE_Damage_C" 1 1)
      (Ability|EndAbility))))

(event Ability|EventOnEndAbility
  (params (bWasCancelled :type Boolean))
  (bind _hitasync_task (Variables|Default|GetHitAsync%20Task))
  (bind _swingasync_task (Variables|Default|GetSwingAsync%20Task))
  (Utilities|IsValid _hitasync_task
    (:Is%20Valid
      (Utilities|IsValid _swingasync_task
        (:Is%20Valid
          (GameplayTasks|EndTask _hitasync_task)
          (GameplayTasks|EndTask _swingasync_task))))))