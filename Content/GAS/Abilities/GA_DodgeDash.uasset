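; Gameplay ability that makes BP_Player dodge-dash with a directional animation and a velocity burst.
; When moving, the player's four dodge direction flags select one of eight in-place montages, and velocity follows the last input vector while keeping vertical speed.
; When stationary, it plays the backward dodge and launches opposite the actor's facing.
; The ability ends after the cooldown delay following a dodge.
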(event Custom|DodgeBackwards
  (bind _dodge_move_distance (Variables|Default|GetDodge%20Move%20Distance))
  (bind _player_movement_comp (Variables|Default|GetPlayer%20Movement%20Comp))
  (bind _returnvalue (Pawn|Components|PawnMovement|GetLastInputVector _player_movement_comp))
  (bind _returnvalue_2 (* _returnvalue _dodge_move_distance))
  (Variables|Default|SetAnim%20Montage "/Game/Animations/RollAndDodge/DodgeAnim/DodgeBackward_Inplace_Retargeted_Montage.DodgeBackward_Inplace_Retargeted_Montage")
  (Animation|PlayAnimMontage (stale Ability|EventActivateAbility _asbp_player) (Variables|Default|GetAnim%20Montage) 1.0 "None")
  (Variables|/Script/Engine.MovementComponent|SetVelocity _player_movement_comp (Math|Vector|MakeVector (.x _returnvalue_2) (.y _returnvalue_2) (.z (Variables|/Script/Engine.MovementComponent|GetVelocity _player_movement_comp))))
  (Utilities|FlowControl|Delay (Variables|Default|GetDodgeCoolDown))
  (Ability|EndAbility))

(event Ability|EventActivateAbility
  (bind _asbp_player (Utilities|Casting|CastToBP_Player (.owneractor (Ability|GetActorInfo)))
    (:then
      (bind _output_get (Variables|Default|SetPlayer%20Movement%20Comp (Pawn|GetMovementComponent _asbp_player)))
      (if (> (Math|Vector|VectorLength (Variables|/Script/Engine.MovementComponent|GetVelocity _output_get)) 0.1)
        (CallFunction|SetDodgeBools (Variables|/Script/MedivalGame.PlayerChar|GetbDodegeForward _asbp_player) (Variables|/Script/MedivalGame.PlayerChar|GetbDodgeBackward _asbp_player) (Variables|/Script/MedivalGame.PlayerChar|GetbDodgeLeft _asbp_player) (Variables|/Script/MedivalGame.PlayerChar|GetbDodgeRight _asbp_player))
        (if (Variables|Default|GetDodgeFwd)
          (if (Variables|Default|GetDodgeRight)
            (Variables|Default|SetAnim%20Montage "/Game/Animations/RollAndDodge/DodgeAnim/DodgeForwardRight_InPlace_Retargeted_Montage.DodgeForwardRight_InPlace_Retargeted_Montage")
            (elif (Variables|Default|GetDodgeLeft)
              (Variables|Default|SetAnim%20Montage "/Game/Animations/RollAndDodge/DodgeAnim/DodgeForwardLeft_InPlace_Retargeted_Montage.DodgeForwardLeft_InPlace_Retargeted_Montage")
              (else
                (Variables|Default|SetAnim%20Montage "/Game/Animations/RollAndDodge/DodgeAnim/DodgeForward_InPlace_Retargeted_Montage.DodgeForward_InPlace_Retargeted_Montage"))))
          (Animation|PlayAnimMontage _asbp_player (Variables|Default|GetAnim%20Montage) 1.0 "None" :!label _label)
          (Variables|/Script/Engine.MovementComponent|SetVelocity (Variables|Default|GetPlayer%20Movement%20Comp) (Math|Vector|MakeVector (.x (* (Pawn|Components|PawnMovement|GetLastInputVector (Variables|Default|GetPlayer%20Movement%20Comp)) (Variables|Default|GetDodge%20Move%20Distance))) (.y (* (Pawn|Components|PawnMovement|GetLastInputVector (Variables|Default|GetPlayer%20Movement%20Comp)) (Variables|Default|GetDodge%20Move%20Distance))) (.z (Variables|/Script/Engine.MovementComponent|GetVelocity (Variables|Default|GetPlayer%20Movement%20Comp)))))
          (Utilities|FlowControl|Delay (Variables|Default|GetDodgeCoolDown))
          (Ability|EndAbility)
          (elif (Variables|Default|GetDodgeBwd)
            (if (Variables|Default|GetDodgeRight)
              (Variables|Default|SetAnim%20Montage "/Game/Animations/RollAndDodge/DodgeAnim/DodgeBackwardRight_InPlace_Retargeted_Montage.DodgeBackwardRight_InPlace_Retargeted_Montage")
              (goto _label)
              (elif (Variables|Default|GetDodgeLeft)
                (Variables|Default|SetAnim%20Montage "/Game/Animations/RollAndDodge/DodgeAnim/DodgeBackwardLeft_InPlace_Retargeted_Montage.DodgeBackwardLeft_InPlace_Retargeted_Montage")
                (goto _label)
                (else
                  (Variables|Default|SetAnim%20Montage "/Game/Animations/RollAndDodge/DodgeAnim/DodgeBackward_Inplace_Retargeted_Montage.DodgeBackward_Inplace_Retargeted_Montage")
                  (goto _label))))
            (elif (Variables|Default|GetDodgeLeft)
              (Variables|Default|SetAnim%20Montage "/Game/Animations/RollAndDodge/DodgeAnim/DodgeLeft_InPlace_Retargeted_Montage.DodgeLeft_InPlace_Retargeted_Montage")
              (goto _label)
              (elif (Variables|Default|GetDodgeRight)
                (Variables|Default|SetAnim%20Montage "/Game/Animations/RollAndDodge/DodgeAnim/DodgeRight_InPlace_Retargeted_Montage.DodgeRight_InPlace_Retargeted_Montage")
                (goto _label)))))
        (else
          (CallFunction|DoBackwardsDodge _asbp_player)
          (Utilities|FlowControl|Delay (Variables|Default|GetDodgeCoolDown))
          (Ability|EndAbility))))
    (:CastFailed
      (Development|PrintString "CAST FAILED IN GA_DODGEDASH !!!!"))))

(event Ability|EventOnEndAbility
  (params (bWasCancelled :type Boolean)))

(fn SetDodgeBools
  (params (DodgeFwd :type Boolean) (DodgeBwd :type Boolean) (DodgeLeft :type Boolean) (DodgeRight :type Boolean))
  (Variables|Default|SetDodgeFwd DodgeFwd)
  (Variables|Default|SetDodgeBwd DodgeBwd)
  (Variables|Default|SetDodgeLeft DodgeLeft)
  (Variables|Default|SetDodgeRight DodgeRight))

(fn DoBackwardsDodge
  (params (Player%20Ref :type BP%20Player%20Object%20Reference))
  (Animation|PlayAnimMontage Player%20Ref "/Game/Animations/RollAndDodge/DodgeAnim/DodgeBackward_Inplace_Retargeted_Montage.DodgeBackward_Inplace_Retargeted_Montage" 1.0 "None")
  (Variables|/Script/Engine.MovementComponent|SetVelocity (Variables|Default|GetPlayer%20Movement%20Comp) (* (* (Transformation|GetActorForwardVector (.owneractor (Ability|GetActorInfo))) -1.0) (Variables|Default|GetDodge%20Move%20Distance))))