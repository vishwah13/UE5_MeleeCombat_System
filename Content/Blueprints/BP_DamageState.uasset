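; Anim notify state that marks the window in an attack animation when the character's sword is active.
; On begin it gets the owning ThirdPersonCharacter, reads the BP_BaseSwordWeapon from its SwordActor child actor and calls SwordActive.
; On end it follows the same cast chain and calls SwordDeactive.
; If either cast fails, the notify does nothing.
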(fn ReceivedNotifyBegin
  (params (MeshComp :type Skeletal%20Mesh%20Component%20Object%20Reference) (Animation :type Anim%20Sequence%20Base%20Object%20Reference) (TotalDuration :type Float%20%28single-precision%29) (EventReference :type Anim%20Notify%20Event%20Reference%20Structure%20%28by%20ref%29))
  (bind _asthird_person_character (Utilities|Casting|CastToThirdPersonCharacter (Components|GetOwner MeshComp)))
  (bind _asbp_base_sword_weapon (Utilities|Casting|CastToBP_BaseSwordWeapon (Variables|/Script/Engine.ChildActorComponent|GetChildActor (Variables|/Game/ThirdPersonBP/Blueprints/ThirdPersonCharacter.ThirdPersonCharacter_C|GetSwordActor _asthird_person_character))))
  (Default|SwordActive _asbp_base_sword_weapon)
  (return false))

(fn ReceivedNotifyEnd
  (params (MeshComp :type Skeletal%20Mesh%20Component%20Object%20Reference) (Animation :type Anim%20Sequence%20Base%20Object%20Reference) (EventReference :type Anim%20Notify%20Event%20Reference%20Structure%20%28by%20ref%29))
  (bind _asthird_person_character (Utilities|Casting|CastToThirdPersonCharacter (Components|GetOwner MeshComp)))
  (bind _asbp_base_sword_weapon (Utilities|Casting|CastToBP_BaseSwordWeapon (Variables|/Script/Engine.ChildActorComponent|GetChildActor (Variables|/Game/ThirdPersonBP/Blueprints/ThirdPersonCharacter.ThirdPersonCharacter_C|GetSwordActor _asthird_person_character))))
  (Default|SwordDeactive _asbp_base_sword_weapon)
  (return false))