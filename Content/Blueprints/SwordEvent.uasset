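; SwordEvent is an animation notify state that switches a character's sword trigger on for a marked window of an animation.
; On begin and end, it casts the mesh owner to CharacterBase and the child actor of its SwordActor component to Sword.
; It calls StartSwordTrigger when the window opens and StopSwordTrigger when it closes, printing a debug message if either cast fails.
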(fn ReceivedNotifyBegin
  (params (MeshComp :type Skeletal%20Mesh%20Component%20Object%20Reference) (Animation :type Anim%20Sequence%20Base%20Object%20Reference) (TotalDuration :type Float%20%28single-precision%29) (EventReference :type Anim%20Notify%20Event%20Reference%20Structure%20%28by%20ref%29))
  (bind _ascharacter_base (Utilities|Casting|CastToCharacterBase (Components|GetOwner MeshComp))
    (:then
      (bind _assword (Utilities|Casting|CastToSword (Variables|/Script/Engine.ChildActorComponent|GetChildActor (Variables|/Script/MedivalGame.CharacterBase|GetSwordActor _ascharacter_base)))
        (:then
          (Class|Sword|StartSwordTrigger _assword)
          (return true))
        (:CastFailed
          (Development|PrintString 0 "CAST FAILED !!!"))))
    (:CastFailed
      (Development|PrintString 0 "CAST  TO PLAYER FAILED !!!"))))

(fn ReceivedNotifyEnd
  (params (MeshComp :type Skeletal%20Mesh%20Component%20Object%20Reference) (Animation :type Anim%20Sequence%20Base%20Object%20Reference) (EventReference :type Anim%20Notify%20Event%20Reference%20Structure%20%28by%20ref%29))
  (bind _ascharacter_base (Utilities|Casting|CastToCharacterBase (Components|GetOwner MeshComp))
    (:then
      (bind _assword (Utilities|Casting|CastToSword (Variables|/Script/Engine.ChildActorComponent|GetChildActor (Variables|/Script/MedivalGame.CharacterBase|GetSwordActor _ascharacter_base)))
        (:then
          (Class|Sword|StopSwordTrigger _assword)
          (return true))
        (:CastFailed
          (Development|PrintString 0 "CAST FAILED !!!"))))
    (:CastFailed
      (Development|PrintString 0 "CAST  TO PLAYER FAILED !!!"))))